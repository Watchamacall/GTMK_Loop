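; BP_MusicInstance manages the game's music across level transitions and also stores a best time per level.
; It spawns the main MetaSound as a persistent 2D sound and keeps the component so level cues can fire one of six trigger parameters, chosen by level index, with a debug print.
; Level-complete audio plays as a separate persistent sound.
; SetBestTime overwrites the level's map entry without comparing times.
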(event Custom|Play%20Main%20Music
  (bind _returnvalue (Audio|SpawnSound2D "/Game/LawrieSounds/Music/Music1/MS_Music1.MS_Music1" 1.0 1.0 0.0 0 true))
  (Variables|Default|SetMusic _returnvalue))

(event Custom|Play%20Level%20Complete
  (Audio|SpawnSound2D "/Game/LawrieSounds/SFX/MS_LevelComplete.MS_LevelComplete" 1.0 1.0 0.0 0 true))

(event Custom|SetBestTime
  (params (Level%20Index :type Integer) (Time :type Float%20%28double-precision%29))
  (bind _leveltimes (Variables|Default|GetLevelTimes))
  (if (Utilities|Map|Contains _leveltimes Level%20Index)
    (Utilities|Map|Remove _leveltimes Level%20Index))
  (Utilities|Map|Add _leveltimes Level%20Index Time))

(event Custom|TriggerLevelMusicCue
  (params (LevelIndex :type Integer))
  (bind _returnvalue (- LevelIndex 1))
  (bind _music (Variables|Default|GetMusic))
  (bind _returnvalue_2 (Utilities|Select :Index _returnvalue :Option%200 "CueMusic_1" :Option%201 "CueMusic_2" :Option%202 "CueMusic_3" :Option%203 "CueMusic_4" :Option%204 "CueMusic_5" :Option%205 "CueMusic_6"))
  (Utilities|IsValid _music
    (:Is%20Valid
      (Class|AudioParameterControllerInterface|SetTriggerParameter _music _returnvalue_2)
      (Development|PrintString (Utilities|String|Append "Triggering music: " (Utilities|String|ToString(Name) _returnvalue_2)) true true "(R=1.000000,G=0.000000,B=0.971273,A=1.000000)" 1e+01))))